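; DialogueSpot is an interaction point that steps through lines of dialogue when the player presses Interact inside its DialogueZone.
; Overlap events from BP_Character toggle an InRange flag that gates the input.
; Each press sets the character's Transition flag and shows the next Texts entry with PrintString.
; A press after the last line resets the index and clears Transition.
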(event OnComponentBeginOverlap(DialogueZone)
  (params (OverlappedComponent :type Primitive%20Component%20Object%20Reference) (OtherActor :type Actor%20Object%20Reference) (OtherComp :type Primitive%20Component%20Object%20Reference) (OtherBodyIndex :type Integer) (bFromSweep :type Boolean) (SweepResult :type Hit%20Result%20Structure%20%28by%20ref%29))
  (Utilities|Casting|CastToBP_Character OtherActor)
  (Variables|Default|SetInRange true))

(event OnComponentEndOverlap(DialogueZone)
  (params (OverlappedComponent :type Primitive%20Component%20Object%20Reference) (OtherActor :type Actor%20Object%20Reference) (OtherComp :type Primitive%20Component%20Object%20Reference) (OtherBodyIndex :type Integer))
  (Utilities|Casting|CastToBP_Character OtherActor)
  (Variables|Default|SetInRange false))

(event EventBeginPlay
  (Variables|Default|SetInRange false)
  (bind _returnvalue (Actor|GetActorOfClass "/Game/Legionary/Blueprints/Character/BP_Character.BP_Character_C"))
  (Variables|Default|Setcharacter _returnvalue))

(event Input|ActionEvents|InputActionInteract
  (params (Key :type Key%20Structure :default "None"))
  (bind _texts (Variables|Default|GetTexts))
  (:Pressed
    (if (Variables|Default|GetInRange)
      (Variables|/Game/Legionary/Blueprints/Character/BP_Character.BP_Character_C|Settransition (Variables|Default|Getcharacter) true)
      (if true
        (if (<= (Utilities|Array|Length _texts) (Variables|Default|GetdialogueIndex))
          (Variables|Default|SetdialogueIndex 0)
          (Variables|/Game/Legionary/Blueprints/Character/BP_Character.BP_Character_C|Settransition (Variables|Default|Getcharacter) false)
          (else
            (Development|PrintString (Utilities|Array|Get(acopy) _texts (Variables|Default|GetdialogueIndex)))
            (Math|Integer|IncrementInt (Variables|Default|GetdialogueIndex))))))))

(fn ConstructionScript)