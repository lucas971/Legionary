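; BP_Arrow is an arrow projectile that damages and knocks back enemy characters.
; It plays a random flight sound on spawn, fading it out when projectile movement stops.
; While moving, its box overlap filters out dashing characters, the owner and non-enemy tags, then decreases health through BP_HealthComponent with normal-based knockback and destroys the arrow.
; The random hit sound is disconnected and never plays.
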(event OnComponentBeginOverlap(Box)
  (params (OverlappedComponent :type Primitive%20Component%20Object%20Reference) (OtherActor :type Actor%20Object%20Reference) (OtherComp :type Primitive%20Component%20Object%20Reference) (OtherBodyIndex :type Integer) (bFromSweep :type Boolean) (SweepResult :type Hit%20Result%20Structure%20%28by%20ref%29))
  (bind _asbp_character (Utilities|Casting|CastToBP_Character OtherActor))
  (if (not (Variables|/Game/Legionary/Blueprints/Character/BP_Character.BP_Character_C|GetisDashing _asbp_character))
    (if (and (== OtherComp (Variables|/Script/Engine.Character|GetCapsuleComponent _asbp_character)) (!= _asbp_character (Components|GetOwner)))
      (if (not (Variables|Default|GethasHit))
        (Utilities|IsValid (Actor|GetComponentbyClass _asbp_character "/Game/Pixel2D/Blueprints/Components/BP_HealthComponent.BP_HealthComponent_C")
          (:Is%20Valid
            (bind _tagcontainer (Class|BPGameplayTagInterface|GetGameplayTagContainer(Message) _asbp_character))
            (if (GameplayTags|HasAnyTags _tagcontainer (Variables|Default|GetenemyTags))
              (if (> (Math|Vector|VectorLength (Variables|/Script/Engine.MovementComponent|GetVelocity (Variables|Default|GetProjectileMovement))) 0.0)
                (Default|DecreaseHealth (Actor|GetComponentbyClass _asbp_character "/Game/Pixel2D/Blueprints/Components/BP_HealthComponent.BP_HealthComponent_C") 1 (* (CallFunction|NormalizedMultiplication (.Normal (Collision|BreakHitResult SweepResult)) (Variables|Default|GetknockbackForce)) (Variables|Default|GetknockbackMultiplier)) (Components|GetOwner))
                (Audio|Components|Audio|Stop (Variables|Default|GetarrowFlySound))
                (Actor|DestroyActor)))))))))

(event OnProjectileStop(ProjectileMovement)
  (params (ImpactResult :type Hit%20Result%20Structure%20%28by%20ref%29))
  (bind _arrowflysound (Variables|Default|GetarrowFlySound)
    (:then
      (Audio|Components|Audio|FadeOut _arrowflysound 0.2 0.0 "Linear" :!class /Script/Engine.AudioComponent))
    (:else)))

(event EventBeginPlay
  (bind _returnvalue (Audio|SpawnSoundatLocation (.OutItem (Utilities|Array|Random (Variables|Default|GetarrowFlySounds))) (Transformation|GetActorLocation) "0, 0, 0" 2.0 1.0 0.5 0 0))
  (Variables|Default|SetarrowFlySound _returnvalue))

(event Collision|EventActorBeginOverlap
  (params (OtherActor :type Actor%20Object%20Reference))
  (|CallParentFunction OtherActor) ; This node is disabled and will not be called.\nDrag off pins to build functionality.
)

(event EventTick
  (params (DeltaSeconds :type Float%20%28single-precision%29))
  (|CallParentFunction DeltaSeconds) ; This node is disabled and will not be called.\nDrag off pins to build functionality.
)

(fn ConstructionScript
  (|CallParentFunction))