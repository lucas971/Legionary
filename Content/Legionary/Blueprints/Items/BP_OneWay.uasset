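; BP_OneWay is a one-way platform item that actors can pass through when JumpThrough is enabled.
; An overlap Box switches the entering actor's capsule response on GameTraceChannel1 to Overlap, then restores it to Block on exit.
; When IsSpear is set, hits on its PaperFlipbook register the platform as SpearPlatform on the hitting BP_Character.
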(event OnComponentBeginOverlap(Box)
  (params (OverlappedComponent :type Primitive%20Component%20Object%20Reference) (OtherActor :type Actor%20Object%20Reference) (OtherComp :type Primitive%20Component%20Object%20Reference) (OtherBodyIndex :type Integer) (bFromSweep :type Boolean) (SweepResult :type Hit%20Result%20Structure%20%28by%20ref%29))
  (bind _returnvalue (Actor|GetComponentbyClass OtherActor "/Script/Engine.CapsuleComponent"))
  ;[1 1 1] COLLISIONS
  (if (Variables|EditableVariables|GetjumpThrough)
    (Utilities|IsValid _returnvalue
      (:Is%20Valid
        (Collision|SetCollisionResponsetoChannel _returnvalue "ECC_GameTraceChannel1" "ECR_Overlap")))))

(event OnComponentEndOverlap(Box)
  (params (OverlappedComponent :type Primitive%20Component%20Object%20Reference) (OtherActor :type Actor%20Object%20Reference) (OtherComp :type Primitive%20Component%20Object%20Reference) (OtherBodyIndex :type Integer))
  (bind _returnvalue (Actor|GetComponentbyClass OtherActor "/Script/Engine.CapsuleComponent"))
  ;[1 1 1] COLLISIONS
  (Utilities|IsValid _returnvalue
    (:Is%20Valid
      (Collision|SetCollisionResponsetoChannel _returnvalue "ECC_GameTraceChannel1" "ECR_Block"))))

(event OnComponentHit(PaperFlipbook)
  (params (HitComponent :type Primitive%20Component%20Object%20Reference) (OtherActor :type Actor%20Object%20Reference) (OtherComp :type Primitive%20Component%20Object%20Reference) (NormalImpulse :type Vector :default "0, 0, 0") (Hit :type Hit%20Result%20Structure%20%28by%20ref%29))
  ;[1 1 1] COLLISIONS
  (if (Variables|EditableVariables|GetisSpear)
    (bind _asbp_character (Utilities|Casting|CastToBP_Character OtherActor))
    (Variables|/Game/Legionary/Blueprints/Character/BP_Character.BP_Character_C|SetSpearPlatform _asbp_character self)))

(fn ConstructionScript)