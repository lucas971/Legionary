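; HealingRock is a healing item that heals a BP_Character entering its trigger, provided the character is below maximum health.
; The trigger overlap checks the HealthComponent, then calls the character's Healing function, which owns the actual heal logic.
; A successful heal also restarts the particle emitter and plays the audio, paused since BeginPlay, from a fixed offset into the sound.
; The rock does not disable or destroy itself after use.
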(event OnComponentBeginOverlap(Trigger)
  (params (OverlappedComponent :type Primitive%20Component%20Object%20Reference) (OtherActor :type Actor%20Object%20Reference) (OtherComp :type Primitive%20Component%20Object%20Reference) (OtherBodyIndex :type Integer) (bFromSweep :type Boolean) (SweepResult :type Hit%20Result%20Structure%20%28by%20ref%29))
  (bind _emitter (Variables|Default|GetEmitter))
  (bind _audio (Variables|Default|GetAudio))
  (bind _asbp_character (Utilities|Casting|CastToBP_Character OtherActor))
  (if (< (Default|GetCurrentHealth (Variables|/Game/Legionary/Blueprints/Character/BP_Character.BP_Character_C|GetHealthComponent _asbp_character)) (Default|GetMaxHealth (Variables|/Game/Legionary/Blueprints/Character/BP_Character.BP_Character_C|GetHealthComponent _asbp_character)))
    (Default|Healing _asbp_character)
    (Niagara|ResetSystem _emitter)
    (Components|Activation|Activate _emitter false)
    (Audio|Components|Audio|Play _audio 7.0)
    (Class|AudioComponent|SetPaused _audio false)))

(event EventBeginPlay
  (Class|AudioComponent|SetPaused (Variables|Default|GetAudio) true))

(fn ConstructionScript)