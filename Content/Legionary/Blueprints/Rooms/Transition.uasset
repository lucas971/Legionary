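; Room transition actor that moves the player from a start trigger to an end arrow when they overlap the trigger.
; It fades the screen out, teleports the character and its camera, applies new X/Z camera bounds, then fades back in while flagging the character as transitioning.
; An optional music request goes to the SoundManager afterwards.
; The construction script labels both ends with the actor's display name.
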(event OnComponentBeginOverlap(StartTrigger)
  (params (OverlappedComponent :type Primitive%20Component%20Object%20Reference) (OtherActor :type Actor%20Object%20Reference) (OtherComp :type Primitive%20Component%20Object%20Reference) (OtherBodyIndex :type Integer) (bFromSweep :type Boolean) (SweepResult :type Hit%20Result%20Structure%20%28by%20ref%29))
  (bind _musicrequest (Variables|Default|GetMusicRequest))
  (bind _asbp_character (Utilities|Casting|CastToBP_Character OtherActor))
  (CameraFades|StartCameraFade :self (Game|GetPlayerCameraManager 0) :ToAlpha 1.0 :Duration 0.25 :bHoldWhenFinished true)
  (Variables|/Game/Legionary/Blueprints/Character/BP_Character.BP_Character_C|SetTransition _asbp_character true)
  (Utilities|FlowControl|Delay 0.25)
  (Transformation|Teleport _asbp_character (Transformation|GetWorldLocation (Variables|Default|GetEndArrow)) (Transformation|GetActorRotation _asbp_character))
  (Default|TeleportCamera (Variables|/Game/Legionary/Blueprints/Character/BP_Character.BP_Character_C|GetCameraController _asbp_character))
  (CallFunction|SetNewBoundaries (Variables|/Game/Legionary/Blueprints/Character/BP_Character.BP_Character_C|GetCameraController _asbp_character))
  (Utilities|FlowControl|Delay 0.5)
  (CameraFades|StartCameraFade :self (Game|GetPlayerCameraManager 0) :FromAlpha 1.0 :Duration 0.5 :bHoldWhenFinished true)
  (Variables|/Game/Legionary/Blueprints/Character/BP_Character.BP_Character_C|SetTransition _asbp_character false)
  (Utilities|IsValid _musicrequest
    (:Is%20Valid
      (bind _returnvalue (Actor|GetActorOfClass "/Game/Legionary/Audio/SoundManager.SoundManager_C"))
      (Default|RequestMusic _returnvalue _musicrequest))))

(fn ConstructionScript
  (Rendering|Components|TextRender|SetText (Variables|Default|GetTextRender) (Utilities|Text|FormatText "{transition ID} End" (Utilities|GetDisplayName self)))
  (Rendering|Components|TextRender|SetText (Variables|Default|GetTextRender1) (Utilities|Text|FormatText "{transition ID} Start" (Utilities|GetDisplayName self))))

(fn SetNewBoundaries
  (params (CameraController :type Camera%20Controller%20Object%20Reference))
  (Variables|/Game/Legionary/Blueprints/Character/CameraController.CameraController_C|SetMinX CameraController (Variables|Default|GetNewMinX))
  (Variables|/Game/Legionary/Blueprints/Character/CameraController.CameraController_C|SetMaxX CameraController (Variables|Default|GetNewMaxX))
  (Variables|/Game/Legionary/Blueprints/Character/CameraController.CameraController_C|SetMinZ CameraController (Variables|Default|GetNewMinZ))
  (Variables|/Game/Legionary/Blueprints/Character/CameraController.CameraController_C|SetMaxZ CameraController (Variables|Default|GetNewMaxZ)))