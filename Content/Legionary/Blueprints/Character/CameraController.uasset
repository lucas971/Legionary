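; Character camera controller that detaches the BP_Character camera and makes it follow on the X/Z plane, side-view style.
; Each Tick measures per-axis distance and direction, then moves the camera within min/max bounds at a fixed Y.
; Per-axis speed is zero near the character, ramps quadratically to the dead zone edge, then linearly to a capped maximum.
; TeleportCamera snaps to the character's X/Z, using a different Y than Tick.
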(event Custom|TeleportCamera
  (bind _character (Variables|Default|GetCharacter))
  (bind _returnvalue (Transformation|GetActorTransform _character))
  (bind _location (Math|Transform|BreakTransform _returnvalue))
  (bind (_x _y _z) (Math|Vector|BreakVector _location))
  ;[1 1 1] Teleport
  (Transformation|SetWorldLocation (Variables|Default|GetCamera) (Math|Vector|MakeVector _x 1e+01 _z) false false))

(event EventBeginPlay
  ;[1 1 1] Init
  (bind _asbp_character (Utilities|Casting|CastToBP_Character (Components|GetOwner)))
  (bind _output_get (Variables|Default|SetCharacter _asbp_character))
  (Variables|Default|SetCamera (Variables|/Game/Legionary/Blueprints/Character/BP_Character.BP_Character_C|GetCamera _output_get))
  (Transformation|DetachFromComponent (Variables|/Game/Legionary/Blueprints/Character/BP_Character.BP_Character_C|GetCamera _output_get) "KeepWorld" "KeepWorld" "KeepWorld" true))

(event EventTick
  (params (DeltaSeconds :type Float%20%28single-precision%29))
  (bind (_returnvalue _right) (Utilities|GetXDistance))
  (bind (_returnvalue_2 _up) (Utilities|GetZDistance))
  (bind _camera (Variables|Default|GetCamera))
  (bind _returnvalue_3 (Utilities|GetXMovement _camera))
  (bind _returnvalue_4 (Utilities|GetZMovement _camera))
  (bind _returnvalue_5 (+ _returnvalue_3 _returnvalue_4))
  (bind (_x _y _z) (Math|Vector|BreakVector _returnvalue_5))
  ;[1 1 1] Getting relative position / distance
  (Variables|Private|SetxDistance _returnvalue)
  (Variables|Private|Setright _right)
  (Variables|Private|SetzDIstance _returnvalue_2)
  (Variables|Private|Setup _up)
  ;[1 1 1] Move camera
  (Transformation|SetWorldLocation _camera (Math|Vector|MakeVector (Math|Float|Min(Float) (Variables|Default|GetMaxX) (Math|Float|Max(Float) (Variables|Default|GetMinX) _x)) 3.3e+04 (Math|Float|Min(Float) (Variables|Default|GetMaxZ) (Math|Float|Max(Float) (Variables|Default|GetMinZ) _z))) false false))