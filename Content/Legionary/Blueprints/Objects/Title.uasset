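; Title is a sprite actor, likely an in-world title graphic, that fades out and removes itself once something overlaps its trigger.
; An overlap on the Trigger component sets a flag with no check on the overlapping actor.
; While flagged, Tick lowers the Paper2D sprite's alpha over about one second, keeping its RGB, then destroys the actor at zero.
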(event OnComponentBeginOverlap(Trigger)
  (params (OverlappedComponent :type Primitive%20Component%20Object%20Reference) (OtherActor :type Actor%20Object%20Reference) (OtherComp :type Primitive%20Component%20Object%20Reference) (OtherBodyIndex :type Integer) (bFromSweep :type Boolean) (SweepResult :type Hit%20Result%20Structure%20%28by%20ref%29))
  (Variables|Default|SetTriggered true))

(event EventBeginPlay
  (Variables|Default|SetTriggered false)
  (Variables|Default|SetCurrentAlpha 1.0))

(event EventTick
  (params (DeltaSeconds :type Float%20%28single-precision%29))
  (bind _papersprite (Variables|Default|GetPaperSprite))
  (bind _spritecolor (Variables|/Script/Paper2D.PaperSpriteComponent|GetSpriteColor _papersprite))
  (bind (_r _g _b) (Math|Color|BreakColor _spritecolor))
  (if (Variables|Default|GetTriggered)
    (bind _output_get (Variables|Default|SetCurrentAlpha (- (Variables|Default|GetCurrentAlpha) DeltaSeconds)))
    (Sprite|SetSpriteColor (Variables|Default|GetPaperSprite) (Math|Color|MakeColor _r _g _b _output_get))
    (if (<= (Variables|Default|GetCurrentAlpha) 0.0)
      (Actor|DestroyActor))))

(fn ConstructionScript)