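; BP_EnemyParent is the base enemy Blueprint in Legionary, handling hurt, death and respawn for a character with a pixel visual component.
; Health changes play a random hurt sound or, below 1, a DoOnce-guarded death that stops movement, spawns sound and particles, and hides the visual.
; RespawnEnemy waits briefly, then restores health, visual and start location and resets the DoOnce.
; Casts on self special-case children: Rook clears EnemyInRange, Wolf skips respawn.
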(event HealthChanged(BP_HealthComponent)
  (params (New%20Value :type Integer) (Change :type E_StatChange%20Enum :default "NewEnumerator0") (Instigator :type Actor%20Object%20Reference))
  ;[1 1 1] check if hurt or dead
  (if (< New%20Value 1)
    (Utilities|FlowControl|DoOnce false
      (:Completed
        (Components|Movement|StopMovementImmediately (Variables|Character|GetCharacterMovement))
        (Variables|Default|SetisDead? true)
        (Components|Timeline|SetLooping (Variables|Default|GetPixelComponent) false)
        (Audio|SpawnSoundatLocation (.OutItem (Utilities|Array|Random (Variables|Default|GetdeathSounds))) (Transformation|GetActorLocation) "0, 0, 0" 0.7 1.0 0.0 0 0)
        (Effects|SpawnEmitteratLocation "/Game/Pixel2D/Particles/P_Death.P_Death" (Transformation|GetActorLocation))
        (Development|SetHiddeninGame (Variables|Default|GetPixelComponent) true false)))
    (else
      (Audio|PlaySoundatLocation (.OutItem (Utilities|Array|Random (Variables|Default|GethurtSounds))) (Transformation|GetActorLocation) "0, 0, 0" 1.0 1.0 0.0 0 0 0))))

(event Custom|RespawnEnemy
  (bind _asbp_rook (Utilities|Casting|CastToBP_Rook self)
    (:then
      (Variables|/Game/Legionary/Blueprints/Enemies/BP_Rook.BP_Rook_C|SetenemyInRange? _asbp_rook false))
    (:CastFailed
      _))
  (Utilities|FlowControl|Delay 2.0)
  ;[1 1 1] respawn
  (Utilities|Casting|CastToBP_Wolf self
    (:CastFailed
      (Variables|Default|SetisDead? false)
      (Components|Timeline|SetLooping (Variables|Default|GetPixelComponent) true)
      (Audio|Components|Audio|Play (Variables|Default|GetPixelComponent))
      (Transformation|Teleport (Variables|Default|GetstartLocation) "0, 0, 0")
      (Development|SetHiddeninGame (Variables|Default|GetPixelComponent) false false)
      (Default|Respawn (Variables|Default|GetBP_HealthComponent))
      ;[1 1 1] check if hurt or dead
      (Utilities|FlowControl|DoOnce false) ; enters at Reset
    )))

(event EventBeginPlay
  (Variables|Default|SetstartLocation (Transformation|GetActorLocation))
  (Development|SetHiddeninGame (Variables|Default|GetPixelComponent) false false))

(event Collision|EventActorBeginOverlap
  (params (OtherActor :type Actor%20Object%20Reference)))

(event EventTick
  (params (DeltaSeconds :type Float%20%28single-precision%29)))

(fn ConstructionScript)