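; Knight enemy AI that patrols waypoints, chases the player inside its sight sphere and attacks in melee.
; A looping timer re-issues move-to-player, while a downward edge trace halts the chase at drops and allows attacks at the goal.
; Notify events fire melee traces from two sockets and reset the attack; stationary knights attack by distance on Tick.
; It flips to face the player, and touching it while not attacking damages the player with knockback.
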(event OnComponentEndOverlap(sightSphere)
  (params (OverlappedComponent :type Primitive%20Component%20Object%20Reference) (OtherActor :type Actor%20Object%20Reference) (OtherComp :type Primitive%20Component%20Object%20Reference) (OtherBodyIndex :type Integer))
  ;[1 1 1] sight sphere
  (Utilities|Casting|CastToBP_Character OtherActor)
  (Variables|Default|SetAs%20BP%20Character 0)
  (if (not (Variables|Default|GetisDead?))
    (if (Variables|EditableVariables|GetcanMove)
      (Utilities|Time|ClearTimerbyFunctionName 0 "MoveToPlayer")
      (AI|Navigation|StopMovement (AI|GetAIController self))
      (Utilities|FlowControl|RetriggerableDelay 2.0)
      (CallFunction|MovetoWaypoint))))

(event OnComponentBeginOverlap(CapsuleComponent)
  (params (OverlappedComponent :type Primitive%20Component%20Object%20Reference) (OtherActor :type Actor%20Object%20Reference) (OtherComp :type Primitive%20Component%20Object%20Reference) (OtherBodyIndex :type Integer) (bFromSweep :type Boolean) (SweepResult :type Hit%20Result%20Structure%20%28by%20ref%29))
  ;[1 1 1] capsule overlap
  (bind _asbp_character (Utilities|Casting|CastToBP_Character OtherActor))
  (if (not (Variables|Default|GetisDead?))
    (if (not (Variables|Booleans|GetisAttacking))
      (bind _result (Default|DecreaseHealth (Variables|/Game/Legionary/Blueprints/Character/BP_Character.BP_Character_C|GetHealthComponent _asbp_character) 1 (* (CallFunction|NormalizedMultiplication (.Normal (Collision|BreakHitResult SweepResult)) (Variables|EditableVariables|GetknockbackForce)) (Variables|Default|GetknockbackMultiplier))))
      (if _result
        (Audio|PlaySoundatLocation (Variables|Default|GethurtSound) (Transformation|GetActorLocation) "0, 0, 0" 3.0 1.0 0.0 0 0 0)))))

(event OnComponentBeginOverlap(sightSphere)
  (params (OverlappedComponent :type Primitive%20Component%20Object%20Reference) (OtherActor :type Actor%20Object%20Reference) (OtherComp :type Primitive%20Component%20Object%20Reference) (OtherBodyIndex :type Integer) (bFromSweep :type Boolean) (SweepResult :type Hit%20Result%20Structure%20%28by%20ref%29))
  ;[1 1 1] sight sphere
  (bind _asbp_character (Utilities|Casting|CastToBP_Character OtherActor))
  (Variables|Default|SetAs%20BP%20Character _asbp_character)
  (if (not (Variables|Default|GetisDead?))
    (if (Variables|EditableVariables|GetcanMove)
      (Utilities|Time|SetTimerbyFunctionName 0 "MoveToPlayer" 0.1 true))))

(event Custom|startAttack_Notify
  ;[1 1 1] spawn melee attack
  (Audio|PlaySoundatLocation (Variables|SFX|GetAttackSound) (Transformation|GetActorLocation) "0, 0, 0" 1.0 1.0 0.0 0 0 0)
  (Default|MeleeTraceAttack (Variables|Default|GetAttackComponent) "HitSocket1" (Variables|Default|GetPixelComponent) (Variables|EditableVariables|Getdamage) (Variables|EditableVariables|GetattackDuration) 0.0 (Variables|EditableVariables|GethitRadius) "(R=1.000000,G=0.000000,B=0.067033,A=1.000000)" (Variables|EditableVariables|GetknockbackForce) (Variables|Tags|GetEnemyTagContainer))
  (Default|MeleeTraceAttack (Variables|Default|GetAttackComponent) "HitSocket2" (Variables|Default|GetPixelComponent) (Variables|EditableVariables|Getdamage) (Variables|EditableVariables|GetattackDuration) 0.0 (Variables|EditableVariables|GethitRadius) "(R=1.000000,G=0.000000,B=0.067033,A=1.000000)" (Variables|EditableVariables|GetknockbackForce) (Variables|Tags|GetEnemyTagContainer)))

(event Custom|endAttack_Notfy
  (Utilities|Time|SetTimerbyFunctionName 0 "MoveToPlayer" 0.1 true)
  (Variables|Booleans|SetisAttacking false)
  (Variables|Booleans|SetattackState false)
  ;[1 1 1] attack player
  (Utilities|FlowControl|DoOnce false) ; enters at Reset
)

(event Custom|moveToWaypoint
  ;[1 1 1] move to waypoint
  (if (not (Variables|Default|GetisDead?))
    (AI|AIMoveTo (AI|GetAIController self) "0, 0, 0" (Utilities|Array|Get(acopy) (Variables|EditableVariables|Getwaypoints) (Variables|Default|GetwaypointIndex)) -1.0 "Default" "Default" true true
      (:OnMoveFinished
        (CallFunction|ReachedWaypoint)))))

(event Custom|reachedWaypoint
  ;[1 1 1] reached waypoint
  (Utilities|FlowControl|RetriggerableDelay 2.0)
  (if (< (Variables|Default|GetwaypointIndex) (- (Utilities|Array|Length (Variables|Default|GetWaypoints)) 1))
    (Math|Integer|IncrementInt (Variables|Default|GetwaypointIndex)
      (:%20%20
        (CallFunction|MovetoWaypoint)))
    (else
      (Variables|Default|SetwaypointIndex 0)
      (CallFunction|MovetoWaypoint))))

(event Custom|attackPlayer
  ;[1 1 1] attack player
  (Utilities|FlowControl|DoOnce false
    (:Completed
      (Utilities|FlowControl|RetriggerableDelay 1.5) ; attack delay
      (Utilities|Time|ClearTimerbyFunctionName 0 "MoveToPlayer")
      (Variables|Booleans|SetisAttacking true)
      (Variables|Booleans|SetattackState true))))

(event Custom|stopAttacking
  ;[1 1 1] stop attacking
  (Variables|Booleans|SetisAttacking false)
  (Variables|Booleans|SetattackState false))

(event Custom|moveToPlayer
  ;[1 1 1] move to player
  (if (not (Variables|Default|GetisDead?))
    (bind _returnvalue (AI|Navigation|MovetoActor (AI|GetAIController (Pawn|GetController)) (Variables|Default|GetAs%20BP%20Character) 55.0 true true true 0))
    (|detectedge "None"
      (:hit
        (if (Utilities|Enum|Equal(Enum) _returnvalue "AlreadyAtGoal")
          (CallFunction|AttackPlayer)
          (else
            (CallFunction|StopAttacking))))
      (:noHit
        (AI|Navigation|StopMovement (AI|GetAIController self))))))

(event EventBeginPlay
  ;[1 1 1] begin play
  (|CallParentFunction)
  (if (Variables|EditableVariables|GetcanMove)
    (CallFunction|MovetoWaypoint)))

(event EventTick
  (params (DeltaSeconds :type Float%20%28single-precision%29))
  ;[1 1 1] tick
  (if (not (Variables|Default|GetisDead?))
    (Variables|Default|GetAs%20BP%20Character
      (:then
        (|Keepplayerinfront)
        (if (not (Variables|EditableVariables|GetcanMove))
          (if (<= (Transformation|GetDistanceTo (Variables|Default|GetAs%20BP%20Character)) 83.0)
            (CallFunction|AttackPlayer)
            (else
              (CallFunction|StopAttacking)))))
      (:else))))

(fn ConstructionScript)

(fn GetEnemyTagContainer
  (return ""))

(fn GetGameplayTagContainer
  (return (Variables|Tags|GetOwnTagContainer)))