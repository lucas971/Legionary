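; BP_Rook1 is an enemy that patrols waypoints and melee-attacks the player character.
; Entering its sight sphere starts a looping timer that halts it, flips it to face the player and raises attack flags after a delay; leaving resumes the patrol.
; An attack notify triggers the melee trace, while capsule contact separately deals damage with knockback.
; The line-of-sight check (DrawPath) is not wired to any event.
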(event OnComponentBeginOverlap(sightSphere)
  (params (OverlappedComponent :type Primitive%20Component%20Object%20Reference) (OtherActor :type Actor%20Object%20Reference) (OtherComp :type Primitive%20Component%20Object%20Reference) (OtherBodyIndex :type Integer) (bFromSweep :type Boolean) (SweepResult :type Hit%20Result%20Structure%20%28by%20ref%29))
  ;[1 1 1] Checks for player
  (bind _asbp_character (Utilities|Casting|CastToBP_Character OtherActor))
  (Variables|Default|SetAs%20BP%20Character _asbp_character)
  (Utilities|Time|SetTimerbyFunctionName 0 "MoveToPlayer" 0.1 true))

(event OnComponentEndOverlap(sightSphere)
  (params (OverlappedComponent :type Primitive%20Component%20Object%20Reference) (OtherActor :type Actor%20Object%20Reference) (OtherComp :type Primitive%20Component%20Object%20Reference) (OtherBodyIndex :type Integer))
  ;[1 1 1] Checks for player
  (bind _asbp_character (Utilities|Casting|CastToBP_Character OtherActor))
  (Variables|Default|SetAs%20BP%20Character _asbp_character)
  (Utilities|Time|ClearTimerbyFunctionName 0 "MoveToPlayer")
  (CallFunction|ResumePath))

(event OnComponentBeginOverlap(CapsuleComponent)
  (params (OverlappedComponent :type Primitive%20Component%20Object%20Reference) (OtherActor :type Actor%20Object%20Reference) (OtherComp :type Primitive%20Component%20Object%20Reference) (OtherBodyIndex :type Integer) (bFromSweep :type Boolean) (SweepResult :type Hit%20Result%20Structure%20%28by%20ref%29))
  ;[1 1 1] damage on overlap
  (bind _asbp_character (Utilities|Casting|CastToBP_Character OtherActor))
  (if (not (Variables|Default|GetisDead?))
    (bind _result (Default|DecreaseHealth (Variables|/Game/Legionary/Blueprints/Character/BP_Character.BP_Character_C|GetHealthComponent _asbp_character) 1 (* (CallFunction|NormalizedMultiplication (.Normal (Collision|BreakHitResult SweepResult)) (Variables|EditableVariables|GetknockbackForce)) (Variables|Default|GetknockbackMultiplier))))
    (if _result
      (Audio|PlaySoundatLocation (Variables|Default|GethurtSound) (Transformation|GetActorLocation) "0, 0, 0" 3.0 1.0 0.0 0 0 0))))

(event Custom|ResumePath
  ;[1 1 1] resume path
  (if (not (Variables|Default|GetisDead?))
    (AI|Navigation|StopMovement (Pawn|GetController) :!pinned true) ; Lost player
    (Utilities|FlowControl|RetriggerableDelay 2.0)
    (Default|StartMove (Variables|Default|GetWaypointMovement) :!pinned true) ; move to waypoint
  ))

(event Custom|MoveToPlayer
  ;[1 1 1] move to player
  (if (not (Variables|Default|GetisDead?))
    (AI|Navigation|StopMovement (Pawn|GetController))
    (|Keepplayerinfront)
    (Utilities|FlowControl|DoOnce false :!label _label
      (:Completed
        (Utilities|FlowControl|RetriggerableDelay 1.0) ; init delay
        (Variables|Booleans|SetisAttacking true)
        (Variables|Booleans|SetattackState true)
        (goto _label Reset)))))

(event Custom|StartAttack_Notify
  ;[1 1 1] attack the player
  (Audio|PlaySoundatLocation (Variables|SFX|GetAttackSound) (Transformation|GetActorLocation) "0, 0, 0" 1.0 1.0 0.0 0 0 0)
  (Default|MeleeTraceAttack (Variables|Default|GetAttackComponent) "HitSocket" (Variables|Default|GetPixelComponent) (Variables|EditableVariables|Getdamage) (Variables|EditableVariables|GetattackDuration) 0.0 (Variables|EditableVariables|GethitRadius) "(R=1.000000,G=0.000000,B=0.067033,A=1.000000)" (Variables|EditableVariables|GetknockbackForce) (Variables|Tags|GetEnemyTagContainer)))

(event EventBeginPlay
  ;[1 1 1] Starts moving
  (|CallParentFunction)
  (Default|StartMove (Variables|Default|GetWaypointMovement))
  (bind _asbp_enemy_attribute (Utilities|Casting|CastToBP_EnemyAttribute (UserInterface|GetUserWidgetObject (Variables|Default|GetWidget))))
  (Variables|/Game/Pixel2D/Blueprints/Widgets/Inventory/BP_EnemyAttribute.BP_EnemyAttribute_C|SetHealthComponent _asbp_enemy_attribute (Variables|Default|GetBP_HealthComponent)))

(event Collision|EventActorBeginOverlap
  (params (OtherActor :type Actor%20Object%20Reference)))

(fn ConstructionScript)

(fn GetEnemyTagContainer
  (return ""))

(fn GetGameplayTagContainer
  (return (Variables|Tags|GetOwnTagContainer)))