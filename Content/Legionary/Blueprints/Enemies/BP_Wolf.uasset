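; BP_Wolf is a werewolf boss on a side-view plane that fights the player, opening ending dialogue on death.
; Once StartFight runs, Tick randomly picks dash or leap after two-second pauses; start/end events gate movement, which a wall box blocks.
; Contact damages the player, while its Damage overlap takes throttled hits with knockback.
; Player death resets position and beginning dialogue; ShouldTUrn's facing comparison is left unconnected.
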(event OnComponentBeginOverlap(CapsuleComponent)
  (params (OverlappedComponent :type Primitive%20Component%20Object%20Reference) (OtherActor :type Actor%20Object%20Reference) (OtherComp :type Primitive%20Component%20Object%20Reference) (OtherBodyIndex :type Integer) (bFromSweep :type Boolean) (SweepResult :type Hit%20Result%20Structure%20%28by%20ref%29))
  (bind _asbp_character (Utilities|Casting|CastToBP_Character OtherActor))
  (if (> (Default|GetCurrentHealth (Variables|Default|GetBP_HealthComponent)) 0)
    (bind _result (Default|DecreaseHealth (Variables|/Game/Legionary/Blueprints/Character/BP_Character.BP_Character_C|GetHealthComponent _asbp_character) 1 (* (CallFunction|NormalizedMultiplication (.Normal (Collision|BreakHitResult SweepResult)) (Variables|Default|GetknockbackForce)) 2.5)))
    (if _result
      _)))

(event OnComponentBeginOverlap(Damage)
  (params (OverlappedComponent :type Primitive%20Component%20Object%20Reference) (OtherActor :type Actor%20Object%20Reference) (OtherComp :type Primitive%20Component%20Object%20Reference) (OtherBodyIndex :type Integer) (bFromSweep :type Boolean) (SweepResult :type Hit%20Result%20Structure%20%28by%20ref%29))
  (Utilities|FlowControl|DoOnce false :!label _label
    (:Completed
      (Default|DecreaseHealth (Variables|Default|GetBP_HealthComponent) 1 (Math|Vector|MakeVector (* (select (> (.X (Math|Vector|BreakVector (Transformation|GetActorLocation (Variables|Default|Getplayer)))) (.X (Math|Vector|BreakVector (Transformation|GetWorldLocation (Variables|Default|GetCapsuleComponent))))) -1 1) 1e+02) 0.0 0.0) OtherActor)
      (Utilities|FlowControl|Delay 0.2)
      (if (> (Default|GetCurrentHealth (Variables|Default|GetBP_HealthComponent)) 0)
        (goto _label Reset)
        (else
          (Default|Initiate (Variables|Default|GetEndingDialogue)))))))

(event OnComponentBeginOverlap(Box)
  (params (OverlappedComponent :type Primitive%20Component%20Object%20Reference) (OtherActor :type Actor%20Object%20Reference) (OtherComp :type Primitive%20Component%20Object%20Reference) (OtherBodyIndex :type Integer) (bFromSweep :type Boolean) (SweepResult :type Hit%20Result%20Structure%20%28by%20ref%29))
  (Variables|Default|SetWall true))

(event OnComponentEndOverlap(Box)
  (params (OverlappedComponent :type Primitive%20Component%20Object%20Reference) (OtherActor :type Actor%20Object%20Reference) (OtherComp :type Primitive%20Component%20Object%20Reference) (OtherBodyIndex :type Integer))
  (Variables|Default|SetWall false))

(event Custom|StartFight
  (Variables|Default|SetFight true)
  (Variables|Default|Settimer 0.0))

(event Custom|PlayerDied
  (if (Variables|Default|GetFight)
    (Variables|Default|SetFight false)
    (Transformation|SetActorLocation (Variables|Default|GetInitialPosition) false true)
    (Variables|/Game/Legionary/Blueprints/Dialogues/DialogueSpot.DialogueSpot_C|SetUsed (Variables|Default|GetBeginningDialogue) false)
    (Variables|Default|SetIsDashing false)
    (Variables|Default|SetIsLeaping false)
    (Variables|Default|SetLookRight true)
    (CallFunction|Rotate)))

(event Custom|Rotate
  (if (Variables|Default|GetLookRight)
    (Transformation|SetActorRotation "0, 0, 0")
    (else
      (Transformation|SetActorRotation "0,180.000000, 0"))))

(event Custom|JumpEnd
  (Variables|Default|SetJumpMovement false)
  (Variables|Default|SetIsLeaping false)
  (Collision|SetCollisionResponsetoChannel (Variables|Default|GetCapsuleComponent) "ECC_GameTraceChannel4" "ECR_Overlap")
  (Audio|PlaySound2D "/Game/Legionary/Audio/SOUND_DESIGN/WEREWOLF/WEREWOLF_JUMP/FEETCrea_Werewolf_jump_LAND_Baum_BaumSFX2021-002.FEETCrea_Werewolf_jump_LAND_Baum_BaumSFX2021-002" 1.0 1.0 0.0 0 0))

(event Custom|DashStart
  (Variables|Default|SetDashMovement true))

(event Custom|DashEnd
  (Variables|Default|SetIsDashing false)
  (Variables|Default|SetDashMovement false))

(event Custom|JumpStart
  (Variables|Default|SetJumpMovement true)
  (Collision|SetCollisionResponsetoChannel (Variables|Default|GetCapsuleComponent) "ECC_GameTraceChannel4" "ECR_Ignore")
  (Audio|PlaySound2D "/Game/Legionary/Audio/SOUND_DESIGN/WEREWOLF/WEREWOLF_JUMP/FEETCrea_Werewolf_jump_Baum_BaumSFX2021-001.FEETCrea_Werewolf_jump_Baum_BaumSFX2021-001" 1.0 1.0 0.0 0 0))

(event EventBeginPlay
  (Variables|Default|SetFight false)
  (Variables|Default|SetInitialPosition (Transformation|GetActorLocation))
  (bind _returnvalue (Actor|GetActorOfClass "/Game/Legionary/Blueprints/Character/BP_Character.BP_Character_C"))
  (Variables|Default|Setplayer _returnvalue)
  (Variables|Default|SetLookRight true)
  (Variables|Default|SetWall false))

(event EventTick
  (params (DeltaSeconds :type Float%20%28single-precision%29))
  (if (not (Math|Boolean|ORBoolean (Variables|Default|GetIsDashing) (Variables|Default|GetIsLeaping) (not (Variables|Default|GetFight))))
    (Variables|Default|Settimer (+ DeltaSeconds (Variables|Default|Gettimer)))
    (if (> (Variables|Default|Gettimer) 2.0)
      (if (Utilities|ShouldTUrn)
        (Variables|Default|SetLookRight (not (Variables|Default|GetLookRight)))
        (CallFunction|Rotate))
      (Variables|Default|Settimer 0.0)
      (if (> (Math|Random|RandomFloat) 0.5)
        (Variables|Default|SetIsDashing true)
        (Audio|PlaySound2D "/Game/Legionary/Audio/SOUND_DESIGN/WEREWOLF/WEREWOLF_GROWL/CREAHmn_WEREWOLF_GROWL_1_Baum_BaumSFX2021.CREAHmn_WEREWOLF_GROWL_1_Baum_BaumSFX2021" 1.0 1.0 0.0 0 0)
        (else
          (Variables|Default|SetIsLeaping true)
          (Audio|PlaySound2D "/Game/Legionary/Audio/SOUND_DESIGN/WEREWOLF/WEREWOLF_GROWL/CREAHmn_WEREWOLF_GROWL_2_Baum_BaumSFX2021.CREAHmn_WEREWOLF_GROWL_2_Baum_BaumSFX2021" 1.0 1.0 0.0 0 0))))
    (elif (Math|Boolean|ANDBoolean (or (Variables|Default|GetDashMovement) (Variables|Default|GetJumpMovement)) (not (Variables|Default|GetWall)) (> (Default|GetCurrentHealth (Variables|Default|GetBP_HealthComponent)) 0))
      (Transformation|SetActorLocation (+ (* (* (Class|KismetMathLibrary|VectorForward) DeltaSeconds) (* (select (Variables|Default|GetLookRight) 1.0 -1.0) (select (Variables|Default|GetJumpMovement) 2e+02 3e+02))) (Transformation|GetActorLocation)) false false))))

(fn ConstructionScript)

(fn GetEnemyTagContainer
  (return ""))

(fn GetGameplayTagContainer
  (return ""))